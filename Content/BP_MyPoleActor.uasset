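; Pole actor that keeps its Pole component vertically in line with its Base component.
; The construction script moves Pole and Base to the actor's X and Y while preserving each one's world height.
; Every Tick, Pole copies Base's world X and Y and keeps its own Z, so it follows Base horizontally only.
; A similar alignment for a Goal component is present but disconnected.
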(event EventBeginPlay)

(event Collision|EventActorBeginOverlap
  (params (OtherActor :type Actor%20Object%20Reference)))

(event EventTick
  (params (DeltaSeconds :type Float%20%28single-precision%29))
  (bind _base (Variables|Default|GetBase))
  (bind _pole (Variables|Default|GetPole))
  (bind _returnvalue (Transformation|GetWorldLocation _base))
  (Transformation|SetWorldLocation _pole (Math|Vector|MakeVector (.x _returnvalue) (.y _returnvalue) (.z (Transformation|GetWorldLocation _pole))) false false))

(fn ConstructionScript
  (bind _returnvalue (Transformation|GetActorLocation))
  (bind _pole (Variables|Default|GetPole))
  (bind _base (Variables|Default|GetBase))
  (Transformation|SetWorldLocation _pole (Math|Vector|MakeVector (.x _returnvalue) (.y _returnvalue) (.z (Transformation|GetWorldLocation _pole))) false false)
  (Transformation|SetWorldLocation _base (Math|Vector|MakeVector (.x _returnvalue) (.y _returnvalue) (.z (Transformation|GetWorldLocation _base))) false false))